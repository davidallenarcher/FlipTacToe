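; A single clickable space on the FlipTacToe board that reports mouse interaction by its Coordinate.
; MouseCollision hover and click call dispatchers with that Coordinate, leaving the response to listeners.
; Helper functions set the Highlight component's material and visibility; BeginPlay and hover end call the material setter with no material supplied.
; BeginPlay also stores a scene component as PieceCenterOfRotation, while Initialize and both player material setters are empty stubs.
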(event OnBeginCursorOver(MouseCollision)
  (params (TouchedComponent :type Primitive%20Component%20Object%20Reference))
  (Default|CallSpaceBeginHover (Variables|Default|GetCoordinate)))

(event OnEndCursorOver(MouseCollision)
  (params (TouchedComponent :type Primitive%20Component%20Object%20Reference))
  (Gameplay|SetHighlightMaterial))

(event OnClicked(MouseCollision)
  (params (TouchedComponent :type Primitive%20Component%20Object%20Reference) (ButtonPressed :type Key%20Structure :default "None"))
  (Default|CallSpaceClickedDispatcher (Variables|Default|GetCoordinate)))

(event EventBeginPlay
  (Variables|Default|SetPieceCenterOfRotation (Variables|Default|GetScene))
  (Gameplay|SetHighlightMaterial))

(fn ConstructionScript)

(fn Initialize)

(fn SetHighlightMaterial
  (params (HighlightMaterial :type Material%20Instance%20Dynamic%20Object%20Reference))
  (Rendering|Material|SetMaterial (Variables|Default|GetHighlight) 0 HighlightMaterial))

(fn SetMatPlayer1
  (params (Material :type Material%20Instance%20Dynamic%20Object%20Reference)))

(fn SetMatPlayer2
  (params (Material :type Material%20Instance%20Dynamic%20Object%20Reference)))

(fn SetHighlightVisibility
  (params (ShouldHighlight :type Boolean))
  (Rendering|SetVisibility (Variables|Default|GetHighlight) ShouldHighlight false))