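; BP_Board is the Flip Tac Toe board actor, holding a 4x4 grid of BP_BoardSpace child actors.
; On BeginPlay it gathers the spaces, calls their player material setters and binds their click and hover events.
; Clicks on empty spaces are relayed through the board's own dispatcher, while hovering one always highlights it as player 1.
; Open, Close and IsOpen use IsOpened on a lazily cached AB_FlipTacToeBoard anim instance.
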(event Custom|SpaceClicked
  (params (Coordinate :type Flip%20Tac%20Toe%20Coordinate%20Structure))
  (bind _returnvalue (Class|FlipTacToeBoard|IsEmptyat Coordinate))
  (if _returnvalue
    (Default|CallSpaceClickedDispatcher Coordinate)))

(event Custom|SpaceBeginHover
  (params (Coordinate :type Flip%20Tac%20Toe%20Coordinate%20Structure))
  (bind _returnvalue (Class|FlipTacToeBoard|IsEmptyat Coordinate))
  (if _returnvalue
    (bind _returnvalue_2 (Class|FlipTacToeBoard|GetSpaceat Coordinate))
    (bind _asbp_board_space (Utilities|Casting|CastToBP_BoardSpace _returnvalue_2))
    (Default|SetHighlight _asbp_board_space true true)))

(event EventBeginPlay
  (CallFunction|AddAlltoSpacesRef)
  (for _array_element (Variables|Default|GetSpaces)
    (Default|SetMatPlayer1 (.AsBP%20Board%20Space (Utilities|Casting|CastToBP_BoardSpace _array_element)))
    (Default|SetMatPlayer2 (.AsBP%20Board%20Space (Utilities|Casting|CastToBP_BoardSpace _array_element)))
    (EventDispatchers|BindEventtoSpaceClickedDispatcher (.AsBP%20Board%20Space (Utilities|Casting|CastToBP_BoardSpace _array_element)) (delegate Custom|SpaceClicked))
    (EventDispatchers|BindEventtoSpaceBeginHover (.AsBP%20Board%20Space (Utilities|Casting|CastToBP_BoardSpace _array_element)) (delegate Custom|SpaceBeginHover))))

(fn ConstructionScript)

(fn IndextoCoordinate
  (params (Index :type Integer))
  (return (Utilities|Struct|MakeFlipTacToeCoordinate (Math|Integer|%(Integer) Index 4) (/ Index 4))))

(fn Open
  (Utilities|IsValid (Variables|Default|GetAnimation%20Instance)
    (:Is%20Valid
      _)
    (:Is%20Not%20Valid
      (bind _asab_flip_tac_toe_board (Utilities|Casting|CastToAB_FlipTacToeBoard (Components|SkeletalMesh|GetAnimInstance (Variables|Default|GetBoardMesh))))
      (Variables|Default|SetAnimation%20Instance _asab_flip_tac_toe_board)))
  (Variables|/Game/FlipTacToe/Animations/AB_FlipTacToeBoard.AB_FlipTacToeBoard_C|SetisOpened (Variables|Default|GetAnimation%20Instance) true))

(fn Close
  (Utilities|IsValid (Variables|Default|GetAnimation%20Instance)
    (:Is%20Valid
      _)
    (:Is%20Not%20Valid
      (bind _asab_flip_tac_toe_board (Utilities|Casting|CastToAB_FlipTacToeBoard (Components|SkeletalMesh|GetAnimInstance (Variables|Default|GetBoardMesh))))
      (Variables|Default|SetAnimation%20Instance _asab_flip_tac_toe_board)))
  (Variables|/Game/FlipTacToe/Animations/AB_FlipTacToeBoard.AB_FlipTacToeBoard_C|SetisOpened (Variables|Default|GetAnimation%20Instance) false))

(fn IsOpen
  (Utilities|IsValid (Variables|Default|GetAnimation%20Instance)
    (:Is%20Valid
      _)
    (:Is%20Not%20Valid
      (bind _asab_flip_tac_toe_board (Utilities|Casting|CastToAB_FlipTacToeBoard (Components|SkeletalMesh|GetAnimInstance (Variables|Default|GetBoardMesh))))
      (Variables|Default|SetAnimation%20Instance _asab_flip_tac_toe_board)))
  (return (Variables|/Game/FlipTacToe/Animations/AB_FlipTacToeBoard.AB_FlipTacToeBoard_C|GetisOpened (Variables|Default|GetAnimation%20Instance))))

(fn AddtoSpacesRef
  (params (SpaceComponentReference :type Child%20Actor%20Component%20Object%20Reference))
  (Utilities|Array|Add (Variables|Default|GetSpaces) (.AsBP%20Board%20Space (Utilities|Casting|CastToBP_BoardSpace (Variables|/Script/Engine.ChildActorComponent|GetChildActor SpaceComponentReference)))))

(fn AddAlltoSpacesRef
  (CallFunction|AddtoSpacesRef (Variables|Default|GetSpace00))
  (CallFunction|AddtoSpacesRef (Variables|Default|GetSpace10))
  (CallFunction|AddtoSpacesRef (Variables|Default|GetSpace20))
  (CallFunction|AddtoSpacesRef (Variables|Default|GetSpace30))
  (CallFunction|AddtoSpacesRef (Variables|Default|GetSpace01))
  (CallFunction|AddtoSpacesRef (Variables|Default|GetSpace11))
  (CallFunction|AddtoSpacesRef (Variables|Default|GetSpace21))
  (CallFunction|AddtoSpacesRef (Variables|Default|GetSpace31))
  (CallFunction|AddtoSpacesRef (Variables|Default|GetSpace02))
  (CallFunction|AddtoSpacesRef (Variables|Default|GetSpace12))
  (CallFunction|AddtoSpacesRef (Variables|Default|GetSpace22))
  (CallFunction|AddtoSpacesRef (Variables|Default|GetSpace32))
  (CallFunction|AddtoSpacesRef (Variables|Default|GetSpace03))
  (CallFunction|AddtoSpacesRef (Variables|Default|GetSpace13))
  (CallFunction|AddtoSpacesRef (Variables|Default|GetSpace23))
  (CallFunction|AddtoSpacesRef (Variables|Default|GetSpace33)))