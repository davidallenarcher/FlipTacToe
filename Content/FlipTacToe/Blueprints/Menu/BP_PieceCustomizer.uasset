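; Menu actor that previews a player's game piece with heads and tails meshes while it is customized through a CustomizePieceWidget.
; On BeginPlay, one dynamic material instance is shared by both meshes and initialized from PlayerPreferences, which also seeds the widget's colors.
; Widget dispatchers update the material's image and base, heads and tails color parameters live.
; SetImages forwards the image choices to the widget.
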(event Custom|Base%20Color%20Changed
  (params (NewColor :type Linear%20Color%20Structure))
  (Rendering|Material|SetVectorParameterValue (Variables|Default|GetMaterialInstance) "BaseColor" NewColor :!class /Script/Engine.MaterialInstanceDynamic))

(event Custom|Heads%20Color%20Changed
  (params (NewColor :type Linear%20Color%20Structure))
  (Rendering|Material|SetVectorParameterValue (Variables|Default|GetMaterialInstance) "HeadsColor" NewColor :!class /Script/Engine.MaterialInstanceDynamic))

(event Custom|Tails%20Color%20Changed
  (params (NewColor :type Linear%20Color%20Structure))
  (Rendering|Material|SetVectorParameterValue (Variables|Default|GetMaterialInstance) "TailsColor" NewColor :!class /Script/Engine.MaterialInstanceDynamic))

(event Custom|Image%20Clicked
  (params (Image :type Texture%202D%20Object%20Reference))
  (Rendering|Material|SetTextureParameterValue (Variables|Default|GetMaterialInstance) "Image" Image))

(event EventBeginPlay
  (bind _playerpreferences (Variables|Default|GetPlayerPreferences))
  (bind _returnvalue (Rendering|Material|CreateDynamicMaterialInstance (Variables|Default|GetTails) 0 0 "None" :!class /Script/Engine.PrimitiveComponent))
  (bind _output_get (Variables|Default|SetMaterialInstance _returnvalue))
  (Rendering|Material|SetMaterial (Variables|Default|GetHeads) 0 _output_get)
  (bind _ascustomize_piece_widget (Utilities|Casting|CastToCustomizePieceWidget (UserInterface|GetWidget (Variables|Default|GetCustomizePieceWidget))))
  (Rendering|Material|SetTextureParameterValue (Variables|Default|GetMaterialInstance) "Image" (.image _playerpreferences))
  (Default|SetInitialBaseColor _ascustomize_piece_widget (.basecolor _playerpreferences))
  (Rendering|Material|SetVectorParameterValue (Variables|Default|GetMaterialInstance) "BaseColor" (.basecolor _playerpreferences) :!class /Script/Engine.MaterialInstanceDynamic)
  (Default|SetInitialHeadsColor _ascustomize_piece_widget (.headscolor _playerpreferences))
  (Rendering|Material|SetVectorParameterValue (Variables|Default|GetMaterialInstance) "HeadsColor" (.headscolor _playerpreferences) :!class /Script/Engine.MaterialInstanceDynamic)
  (Default|SetInitialTailsColor _ascustomize_piece_widget (.tailscolor _playerpreferences))
  (Rendering|Material|SetVectorParameterValue (Variables|Default|GetMaterialInstance) "TailsColor" (.tailscolor _playerpreferences) :!class /Script/Engine.MaterialInstanceDynamic)
  (EventDispatchers|BindEventtoImageClickedDispatcher _ascustomize_piece_widget (delegate Custom|Image%20Clicked))
  (EventDispatchers|BindEventtoBaseColorChangedDispatcher _ascustomize_piece_widget (delegate Custom|Base%20Color%20Changed))
  (EventDispatchers|BindEventtoHeadsColorChangedDispatcher _ascustomize_piece_widget (delegate Custom|Heads%20Color%20Changed))
  (EventDispatchers|BindEventtoTailsColorChangedDispatcher _ascustomize_piece_widget (delegate Custom|Tails%20Color%20Changed)))

(fn ConstructionScript)

(fn SetImages
  (params (Images :type Array%20of%20Texture%202D%20Object%20References))
  (Default|SetImages (.AsCustomize%20Piece%20Widget (Utilities|Casting|CastToCustomizePieceWidget (UserInterface|GetWidget (Variables|Default|GetCustomizePieceWidget)))) Images))