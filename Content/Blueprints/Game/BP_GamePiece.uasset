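; BP_GamePiece is a game piece actor that flips 180 degrees up, right, down or left.
; The Flip event plays a timeline that feeds its progress and the direction into SetRotation.
; Above a threshold, SetRotation shifts CenterOfRotation toward that direction, counter-offsets the mesh, then rolls or pitches around that shifted pivot.
; The construction script calls the same function to pose the piece from its variables.
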(event Custom|Flip
  (params (PieceFlipDirection :type GameDirection%20Enum :default "UP"))
  (bind _rotationamount (Timeline|HorizontalFlipTimeline Play)
    (:Update
      (CallFunction|SetRotation _rotationamount PieceFlipDirection))))

(fn ConstructionScript
  (CallFunction|SetRotation (Variables|Default|GetRotationAmount) (Variables|Default|GetDirection)))

(fn SetRotation
  (params (RotationAmount :type Float%20%28single-precision%29) (Direction :type GameDirection%20Enum :default "UP"))
  (if (> RotationAmount (LocalVariables|GetThreshold))
    (switch Utilities|FlowControl|Switch|SwitchonGameDirection Direction
      (:UP
        (LocalVariables|SetVerticalRotationMultiplier 1.0)
        (LocalVariables|SetHorizontalRotationMultiplier 0.0))
      (:Right
        (LocalVariables|SetVerticalRotationMultiplier 0.0)
        (LocalVariables|SetHorizontalRotationMultiplier 1.0))
      (:Down
        (LocalVariables|SetVerticalRotationMultiplier -1.0)
        (LocalVariables|SetHorizontalRotationMultiplier 0.0))
      (:Left
        (LocalVariables|SetVerticalRotationMultiplier 0.0)
        (LocalVariables|SetHorizontalRotationMultiplier -1.0)))
    (Transformation|SetRelativeLocation (Variables|Default|GetCenterOfRotation) (Math|Vector|MakeVector (* (LocalVariables|GetHorizontalRotationMultiplier) 1.25) (* (LocalVariables|GetVerticalRotationMultiplier) -1.25) 0.0) false false)
    (Transformation|SetRelativeLocation (Variables|Default|GetPieceMeshComponent) (Math|Vector|MakeVector (* (LocalVariables|GetHorizontalRotationMultiplier) -1.25) (* (LocalVariables|GetVerticalRotationMultiplier) 1.25) 0.0) false false)
    (Transformation|SetRelativeRotation (Variables|Default|GetCenterOfRotation) (Math|Rotator|MakeRotator (* RotationAmount (LocalVariables|GetVerticalRotationMultiplier) -1.8e+02) (* RotationAmount (LocalVariables|GetHorizontalRotationMultiplier) -1.8e+02) 0.0) false false)))