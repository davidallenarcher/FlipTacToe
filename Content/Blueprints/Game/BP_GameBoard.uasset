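; BP_GameBoard is the 4x4 FlipTacToe board actor, with two doors that OpenBoard rotates by a given amount.
; On BeginPlay it spawns a hidden highlight mesh for each space, attached to the board.
; SetHoveredSpace shows only the hovered space's mesh, and ClearHoverSpace hides them all.
; Helper functions convert between array index, grid coordinate and position on the board, with a validity check for incoming positions.
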(event Custom|OpenBoard
  (params (OpenAmount :type Float%20%28single-precision%29))
  (Transformation|SetRelativeRotation (Variables|Default|GetDoorLeft) (Math|Rotator|MakeRotator 0.0 OpenAmount 0.0) false false)
  (Transformation|SetRelativeRotation (Variables|Default|GetDoorRight) (Math|Rotator|MakeRotator 0.0 OpenAmount 1.8e+02) false false))

(event EventBeginPlay
  (Private|Initializations|InitHoverSpaces))

(fn ConstructionScript)

(fn InitHoverSpaces
  (Utilities|Array|Clear (Variables|Default|GetSpaceMeshes))
  (for _index (range 0 15)
    (bind _output_get (LocalVariables|SetIndex _index))
    (bind _returnvalue (AddComponent|AddStaticMeshComponent true (Math|Transform|MakeTransform (CallFunction|BoardCoordinatetoWorldCoordinate (Utilities|IndextoCoordinate _output_get)) "0, 0, 0" "1,1,1")))
    (bind _output_get_2 (LocalVariables|SetSpace _returnvalue))
    (Utilities|Array|Add (Variables|Default|GetSpaceMeshes) _output_get_2)
    (Transformation|AttachComponentToComponent (LocalVariables|GetSpace) (Variables|Default|GetBoard) "None" "KeepRelative" "KeepRelative" "KeepRelative" true)
    (Components|StaticMesh|SetStaticMesh (LocalVariables|GetSpace) "/Game/Meshes/FlipTacToePiece.FlipTacToePiece")
    (Development|SetHiddeninGame (LocalVariables|GetSpace) true false)
    (Rendering|Material|SetMaterial (LocalVariables|GetSpace) 0 "/Game/Materials/MAT_Space.MAT_Space")))

(fn SetHoveredSpace
  (params (GameCoordinate :type Game%20Coordinate%20Structure%20%28by%20ref%29))
  (LocalVariables|SetHoveredIndex (Utilities|CoordinatetoIndex GameCoordinate))
  (for (_array_element _array_index) (Variables|Default|GetSpaceMeshes)
    (Development|SetHiddeninGame _array_element (!= _array_index (LocalVariables|GetHoveredIndex)) false)))

(fn ClearHoverSpace
  (for _array_element (Variables|Default|GetSpaceMeshes)
    (Development|SetHiddeninGame _array_element true false)))

(fn WorldCoordinatetoBoardCoordinate
  (params (WorldCoordinate :type Vector))
  (bind _board (Utilities|WorldtoBoard (.y WorldCoordinate)))
  (bind _board_2 (Utilities|WorldtoBoard (.x WorldCoordinate)))
  (bind _gamecoordinate (Utilities|Struct|MakeGameCoordinate _board_2 _board))
  (return (Class|GameBoard|IsValidSpace _gamecoordinate) _gamecoordinate))

(fn BoardCoordinatetoWorldCoordinate
  (params (BoardCoordinate :type Game%20Coordinate%20Structure))
  (return (Math|Vector|MakeVector (Utilities|BoardtoWorld (.column BoardCoordinate)) (Utilities|BoardtoWorld (.row BoardCoordinate)) 0.0)))