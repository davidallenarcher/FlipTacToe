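; Player controller for the local multiplayer level that sets up the player's HUD.
; On BeginPlay it creates a PlayerHUD widget, adds it to the viewport and sets its instruction text to a waiting-for-opponent message.
; It then switches to game-only input with the mouse cursor visible; an unconnected Game-and-UI input alternative never runs.
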(event EventBeginPlay
  (bind _returnvalue (UserInterface|CreateWidget "/Game/Blueprints/Widgets/PlayerHUD.PlayerHUD_C" self))
  (bind _output_get (Variables|Default|SetPlayerHUD _returnvalue))
  (UserInterface|Viewport|AddtoViewport _output_get 0)
  (Variables|/Game/Blueprints/Widgets/PlayerHUD.PlayerHUD_C|SetInstructionValue (Variables|Default|GetPlayerHUD) "Waiting for opponent to join session")
  (Input|SetInputModeGameOnly self)
  (Variables|/Script/Engine.PlayerController|SetbShowMouseCursor self true))

(event EventTick
  (params (DeltaSeconds :type Float%20%28single-precision%29)))

(fn ConstructionScript)