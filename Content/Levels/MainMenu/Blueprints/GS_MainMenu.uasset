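; GS_MainMenu is the main menu's controller for a board game, animating the level's BP_GameBoard and launching local or LAN multiplayer.
; Timelines drive the board's OpenBoard for opening and closing, with local play opening PieceSettings after the close.
; Hosting creates a two-player LAN session alongside the animation, opening NetworkMultiplayer as a listen server once both complete.
; Joining searches LAN sessions, then closes the board and joins the first result.
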(event Custom|OpenBoard
  (bind _openpercentage (Timeline|Board%20Open%20Timeline Play)
    (:Update
      (Default|OpenBoard (Variables|Default|GetGameBoard) _openpercentage))))

(event Custom|Start%20Local%20Multiplayer
  (bind _openpercentage (Timeline|Close%20Board%20Timeline Play)
    (:Update
      (Default|OpenBoard (Variables|Default|GetGameBoard) (* _openpercentage 1.8e+02)))
    (:Finished
      (Game|OpenLevel(byName) "PieceSettings"))))

(event Custom|Host%20Network%20Multiplayer
  (|Session (Game|GetPlayerController 0) 2 true
    (:then
      (bind _openpercentage (Timeline|Close%20Board%20Timeline%202 Play)
        (:Update
          (Default|OpenBoard (Variables|Default|GetGameBoard) (* _openpercentage 1.8e+02)))
        (:Finished
          (bind _output_get (Variables|Default|SetIsAnimationFinished true))
          (if (and _output_get (stale _output_get_2)) :!label _label
            (Game|OpenLevel(byName) "NetworkMultiplayer" true "listen")))))
    (:OnSuccess
      (bind _output_get_2 (Variables|Default|SetIsSessionCreated true))
      (goto _label))))

(event Custom|Join%20Network%20Multiplayer
  (bind _results (|FindSessions (Game|GetPlayerController 0) 10 true)
    (:OnSuccess
      (bind _openpercentage (Timeline|Close%20Board%20Timeline%203 Play)
        (:Update
          (Default|OpenBoard (Variables|Default|GetGameBoard) (* _openpercentage 1.8e+02)))
        (:Finished
          (|JoinSession (Game|GetPlayerController 0) (Utilities|Array|Get(acopy) _results)))))))

(event EventBeginPlay
  (bind _returnvalue (Actor|GetActorOfClass "/Game/Blueprints/Game/BP_GameBoard.BP_GameBoard_C"))
  (Variables|Default|SetGameBoard _returnvalue))

(fn ConstructionScript)