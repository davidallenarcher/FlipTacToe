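; Player controller for the main menu that switches between a pulsing "Press Any Key" prompt and the start-game buttons.
; On BeginPlay, the local controller enables the cursor and Game-and-UI input, then creates the menu widget with both elements hidden.
; A timeline pulses the prompt's opacity until a key press reveals the buttons.
; Each press restarts a retriggerable delay that brings the prompt back after a minute of inactivity.
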(event Custom|Set%20Press%20Any%20Key%20Opacity
  (params (InOpacity :type Float%20%28single-precision%29))
  (Widget|SetRenderOpacity (Variables|/Game/Levels/MainMenu/Widgets/Widget_MainMenu.Widget_MainMenu_C|GetPressAnyKey (Variables|Default|GetMainMenu)) InOpacity))

(event Custom|Start%20Showing%20Press%20Any%20Key
  ;[1 1 1] Show "Press Any Key" on main menu
  (CallFunction|HideMainMenu)
  (Variables|Default|SetShowing%20Press%20Any%20Key? true)
  (bind _anykeyopacity (Timeline|Pulse%20Press%20Any%20Key Play)
    (:Update
      (CallFunction|SetPressAnyKeyOpacity _anykeyopacity))))

(event Custom|Stop%20Showing%20Press%20Any%20Key
  ;[1 1 1] Show "Press Any Key" on main menu
  (CallFunction|ShowMainMenu)
  (Variables|Default|SetShowing%20Press%20Any%20Key? false)
  (Utilities|FlowControl|Sequence
    (:then_0
      (bind _anykeyopacity (Timeline|Pulse%20Press%20Any%20Key Stop)
        (:Update
          (CallFunction|SetPressAnyKeyOpacity _anykeyopacity))))
    (:then_1
      (CallFunction|SetPressAnyKeyOpacity 0.0))))

(event Custom|Show%20Main%20Menu
  (bind _mainmenu (Variables|Default|GetMainMenu))
  (bind _startgamebuttons (Variables|/Game/Levels/MainMenu/Widgets/Widget_MainMenu.Widget_MainMenu_C|GetStartGameButtons _mainmenu))
  (Widget|SetRenderOpacity _startgamebuttons 1.0)
  (Widget|SetIsEnabled _startgamebuttons true))

(event Custom|Hide%20Main%20Menu
  (bind _mainmenu (Variables|Default|GetMainMenu))
  (bind _startgamebuttons (Variables|/Game/Levels/MainMenu/Widgets/Widget_MainMenu.Widget_MainMenu_C|GetStartGameButtons _mainmenu))
  (Widget|SetRenderOpacity _startgamebuttons 0.0)
  (Widget|SetIsEnabled _startgamebuttons false))

(event EventBeginPlay
  (if (Pawn|IsLocalController)
    (Utilities|FlowControl|Sequence
      (:then_0
        (Input|SetInputModeGameandUI self 0 "DoNotLock" false)
        (Variables|Default|SetbShowMouseCursor true))
      (:then_1
        (bind _returnvalue (UserInterface|CreateWidget "/Game/Levels/MainMenu/Widgets/Widget_MainMenu.Widget_MainMenu_C" self))
        (bind _output_get (Variables|Default|SetMainMenu _returnvalue))
        (UserInterface|Viewport|AddtoViewport _output_get 0))
      (:then_2
        (Widget|SetRenderOpacity (Variables|/Game/Levels/MainMenu/Widgets/Widget_MainMenu.Widget_MainMenu_C|GetPressAnyKey (Variables|Default|GetMainMenu)) 0.0))
      (:then_3
        (Widget|SetRenderOpacity (Variables|/Game/Levels/MainMenu/Widgets/Widget_MainMenu.Widget_MainMenu_C|GetStartGameButtons (Variables|Default|GetMainMenu)) 0.0)
        (Widget|SetIsEnabled (Variables|/Game/Levels/MainMenu/Widgets/Widget_MainMenu.Widget_MainMenu_C|GetStartGameButtons (Variables|Default|GetMainMenu)) false))
      (:then_4)
      (:then_5))))

(event Input|KeyboardEvents|AnyKey
  (params (Key :type Key%20Structure))
  (:Pressed
    (if (Variables|Default|GetShowing%20Press%20Any%20Key?)
      (CallFunction|StopShowingPressAnyKey))
    (Utilities|FlowControl|RetriggerableDelay 6e+01)
    (CallFunction|StartShowingPressAnyKey)))

(fn ConstructionScript)