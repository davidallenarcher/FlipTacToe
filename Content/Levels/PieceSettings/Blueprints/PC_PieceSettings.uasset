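; Player controller for the piece settings level, meant to link a PieceSettings widget to a display piece with base color and heads/tails colors and icons.
; BeginPlay only sets Game and UI input and shows the cursor.
; Five change events forward new values to the matching PieceDisplay setters.
; The chain that creates the widget, binds those events and finds the BP_PieceSettings actor as PieceDisplay is disconnected, so never runs.
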(event Custom|BaseColorChanged
  (params (NewBaseColor :type Linear%20Color%20Structure))
  (Default|SetBaseColor (Variables|Default|GetPieceDisplay) NewBaseColor))

(event Custom|HeadsColorChanged
  (params (NewHeadsColor :type Linear%20Color%20Structure))
  (Default|SetHeadsColor (Variables|Default|GetPieceDisplay) NewHeadsColor))

(event Custom|TailsColorChanged
  (params (NewTailsColor :type Linear%20Color%20Structure))
  (Default|SetTailsColor (Variables|Default|GetPieceDisplay) NewTailsColor))

(event Custom|HeadsIconChanged
  (params (NewHeadsIcon :type Texture%20Object%20Reference))
  (Default|SetHeadsIcon (Variables|Default|GetPieceDisplay) NewHeadsIcon))

(event Custom|TailsIconChanged
  (params (NewTailsIcon :type Texture%20Object%20Reference))
  (Default|SetTailsIcon (Variables|Default|GetPieceDisplay) NewTailsIcon))

(event EventBeginPlay
  (Input|SetInputModeGameandUI self 0 "DoNotLock" true)
  (Variables|/Script/Engine.PlayerController|SetbShowMouseCursor self true))

(fn ConstructionScript)