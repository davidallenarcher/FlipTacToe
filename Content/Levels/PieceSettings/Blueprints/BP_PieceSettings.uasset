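; Level actor that previews one player's piece, with a settings widget for customizing its colors and heads/tails icons.
; On BeginPlay it creates a dynamic material instance, binds to the widget's update events and seeds the widget with its default values.
; Setter events write material parameters on the constantly spinning mesh.
; Only base color changes are also saved to the game instance, as Player 1 or 2 by PlayerIndex.
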(event Custom|SetBaseColor
  (params (NewBaseColor :type Linear%20Color%20Structure))
  (Variables|Default|SetBaseColor NewBaseColor)
  (Rendering|Material|SetVectorParameterValue (Variables|Default|GetPieceMaterialInstance) "BaseColor" (Variables|Default|GetBaseColor) :!class /Script/Engine.MaterialInstanceDynamic)
  (Variables|Default|GetBPGameInstance
    (:then
      (switch int (Variables|Default|GetPlayerIndex)
        (:Default
          (Variables|/Game/Blueprints/Engine/BP_GameInstance.BP_GameInstance_C|SetPlayer2BaseColor (Variables|Default|GetBPGameInstance) (Variables|Default|GetBaseColor)))
        (:0
          (Variables|/Game/Blueprints/Engine/BP_GameInstance.BP_GameInstance_C|SetPlayer1BaseColor (Variables|Default|GetBPGameInstance) (Variables|Default|GetBaseColor)))))
    (:else)))

(event Custom|setHeadsColor
  (params (NewHeadsColor :type Linear%20Color%20Structure))
  (Rendering|Material|SetVectorParameterValue (Variables|Default|GetPieceMaterialInstance) "HeadsColor" NewHeadsColor :!class /Script/Engine.MaterialInstanceDynamic))

(event Custom|setTailsColor
  (params (NewTailsColor :type Linear%20Color%20Structure))
  (Rendering|Material|SetVectorParameterValue (Variables|Default|GetPieceMaterialInstance) "TailsColor" NewTailsColor :!class /Script/Engine.MaterialInstanceDynamic))

(event Custom|SetTailsIcon
  (params (NewTailsIcon :type Texture%20Object%20Reference))
  (Rendering|Material|SetTextureParameterValue (Variables|Default|GetPieceMaterialInstance) "TailsIcon" NewTailsIcon))

(event Custom|SetHeadsIcon
  (params (NewHeadsIcon :type Texture%20Object%20Reference))
  (Rendering|Material|SetTextureParameterValue (Variables|Default|GetPieceMaterialInstance) "HeadsIcon" NewHeadsIcon))

(event EventBeginPlay
  (bind _returnvalue (Rendering|Material|CreateDynamicMaterialInstance (Rendering|Material|GetMaterial (Variables|Default|GetPieceMesh) 0) "None" "None" :!class /Script/Engine.KismetMaterialLibrary))
  (bind _output_get (Variables|Default|SetPieceMaterialInstance _returnvalue))
  (Rendering|Material|SetMaterial (Variables|Default|GetPieceMesh) 0 _output_get)
  (bind _aspiece_settings_widget (Utilities|Casting|CastToPieceSettingsWidget (UserInterface|GetWidget (Variables|Default|GetPieceSettings))))
  (Variables|Default|SetPiece%20Settings%20Widget _aspiece_settings_widget)
  (EventDispatchers|BindEventtoBaseColorUpdated (Variables|Default|GetPiece%20Settings%20Widget) (EventDispatchers|CreateEvent :!event Custom|SetBaseColor))
  (EventDispatchers|BindEventtoHeadsColorUpdated (Variables|Default|GetPiece%20Settings%20Widget) (EventDispatchers|CreateEvent :!event Custom|setHeadsColor))
  (EventDispatchers|BindEventtoTailsColorUpdated (Variables|Default|GetPiece%20Settings%20Widget) (EventDispatchers|CreateEvent :!event Custom|setTailsColor))
  (EventDispatchers|BindEventtoHeadsIconUpdated (Variables|Default|GetPiece%20Settings%20Widget) (EventDispatchers|CreateEvent :!event Custom|SetHeadsIcon))
  (EventDispatchers|BindEventtoTailsIconUpdated (Variables|Default|GetPiece%20Settings%20Widget) (EventDispatchers|CreateEvent :!event Custom|SetTailsIcon))
  (Default|SetBaseColor (Variables|Default|GetPiece%20Settings%20Widget) (Variables|Default|GetBaseColor))
  (Default|SetHeadsColor (Variables|Default|GetPiece%20Settings%20Widget) (Variables|Default|GetHeadsColor))
  (Default|SetTailsColor (Variables|Default|GetPiece%20Settings%20Widget) (Variables|Default|GetTailsColor))
  (Default|SetHeadsIconIndex (Variables|Default|GetPiece%20Settings%20Widget) (Variables|Default|GetHeadsIconIndex))
  (Default|SetTailsIconIndex (Variables|Default|GetPiece%20Settings%20Widget) (Variables|Default|GetTailsIconIndex))
  (bind _asbp_game_instance (Utilities|Casting|CastToBP_GameInstance (Game|GetGameInstance)))
  (Variables|Default|SetBPGameInstance _asbp_game_instance))

(event EventTick
  (params (DeltaSeconds :type Float%20%28single-precision%29))
  (Transformation|AddLocalRotation (Variables|Default|GetPieceMesh) (Math|Rotator|MakeRotator 0.0 (* DeltaSeconds -9e+01) 0.0) false false))

(fn ConstructionScript)