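; Pawn for the PieceSettings level that adapts its spring arm to the viewport's shape.
; Every Tick it feeds the viewport's height-to-width ratio into a fitted reciprocal curve, A / (X + B) + C, to set the arm length.
; A Max clamp keeps the arm from getting shorter than a fixed minimum.
; BeginPlay and the construction script are empty.
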(event EventBeginPlay)

(event EventTick
  (params (DeltaSeconds :type Float%20%28single-precision%29))
  (bind _returnvalue (Viewport|GetViewportSize))
  (Variables|/Script/Engine.SpringArmComponent|SetTargetArmLength (Variables|Default|GetSpringArm) (Math|Float|Max(Float) (|((a/(x+b))+c) 4.08106 (/ (.y _returnvalue) (.x _returnvalue)) -0.015439 7.8874) 12.8)))

(fn ConstructionScript)