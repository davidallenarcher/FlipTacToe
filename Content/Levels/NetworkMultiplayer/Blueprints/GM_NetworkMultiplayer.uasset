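; Game mode for the network multiplayer level that assigns a PlayerStart to each player.
; ChoosePlayerStart indexes the level's PlayerStart actors by the current player count, without bounds checking; it calls GetMyPlayerIndex but ignores the result.
; BeginPlay only calls its parent, and disconnected logic for finding and opening BP_GameBoard never runs.
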(event EventBeginPlay
  (|CallParentFunction))

(fn ConstructionScript)

(fn ChoosePlayerStart
  (params (Player :type Controller%20Object%20Reference))
  (bind _asplayer_controller (Utilities|Casting|CastToPlayerController Player))
  (Class|TurnBasedBlueprintLibrary|GetMyPlayerIndex _asplayer_controller)
  (bind _outactors (Actor|GetAllActorsOfClass "/Script/Engine.PlayerStart"))
  (bind _returnvalue (Class|GameModeBase|GetNumPlayers))
  (return (Utilities|Array|Get(acopy) _outactors _returnvalue)))