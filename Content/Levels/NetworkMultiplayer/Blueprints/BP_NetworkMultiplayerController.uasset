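; Player controller for networked FlipTacToe that creates the local HUD, shows phase instructions and handles board and camera input.
; The current player phase drives per-tick hover highlighting of valid spaces, queried from the game state and board, and Select passes the hovered space to HandleSpaceSelect.
; Holding MoveCamera re-centers the hidden cursor and enables pawn rotation and pitch, while zoom always works.
; A Server RPC ends the turn through the game state.
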(event EventBeginPlay
  (bind _self self)
  (bind _returnvalue (Utilities|GetDisplayName _self))
  (if (Pawn|IsLocalController)
    (Development|PrintString (Utilities|String|Append "BP_PlayerController(local): " _returnvalue) true true "(R=0.000000,G=0.660000,B=1.000000,A=1.000000)" 1.2e+02)
    (bind _returnvalue_2 (UserInterface|CreateWidget "/Game/Blueprints/Widgets/PlayerHUD.PlayerHUD_C" self))
    (bind _output_get (Variables|Default|SetPlayerHUD _returnvalue_2))
    (UserInterface|Viewport|AddtoViewport _output_get 0)
    (else
      (Development|PrintString (Utilities|String|Append "BP_PlayerController(Remote): " _returnvalue) true true "(R=0.000000,G=0.660000,B=1.000000,A=1.000000)" 1.2e+02))))

(event EventTick
  (params (DeltaSeconds :type Float%20%28single-precision%29))
  (bind (_game_state _bsuccess) (CallFunction|GetFlipTacToeGameState))
  (|CenterMouse
    (:OutputPin
      (Utilities|SwitchGamePhase
        (:Winner
          (if _bsuccess :!label _label
            (Default|SetHoverSpace _game_state false)))
        (:Loser
          (goto _label))
        (:Waiting%20for%20other%20player
          (goto _label))
        (:Select%20opponent%20piece
          (CallFunction|TickHoverSpace :!label _label_2))
        (:Flip%20opponent%20piece
          (goto _label_2))
        (:Place%20own%20piece
          (goto _label_2))))))

(event EventOnPlayerPhaseChanged
  (params (NewPlayerPhase :type PlayerPhase%20Enum :default "Winner"))
  (bind _playerhud (Variables|Default|GetPlayerHUD)
    (:then
      (Variables|/Game/Blueprints/Widgets/PlayerHUD.PlayerHUD_C|SetInstructionValue _playerhud (Utilities|Select :Index (Variables|Default|GetCurrentPlayerPhase) :Winner "YOU WIN!" :Loser "Sorry, Better Luck Next Time" :WaitingForOpponent "Waiting For Opponent" :SelectOpponentPiece "Select Opponents Piece To Flip" :FlipOpponentPiece "Select Adjactent Empty Space To Flip  Into" :PlaceOwnPiece "Select An Empty Space To Place Your Piece" :SelectFace "")))
    (:else
      (Development|PrintString "HUD Unavailable"))))

(event Custom|End%20Turn%20%28server%29
  (Class|FTTMultiplayerGameState|EndPlayerTurnServer (.Game%20State (CallFunction|GetFlipTacToeGameState))))

(event Input|ActionEvents|InputActionMoveCamera
  (params (Key :type Key%20Structure))
  (:Pressed
    (Variables|Default|SetMovingCamera? true)
    (Variables|Default|SetbShowMouseCursor false)
    (Input|SetInputModeGameOnly self))
  (:Released
    (Variables|Default|SetMovingCamera? false)
    (Variables|Default|SetbShowMouseCursor true)
    (Input|SetInputModeGameandUI self 0 "DoNotLock" false)))

(event Input|ActionEvents|InputActionSelect
  (params (Key :type Key%20Structure))
  (:Pressed
    (bind (_returnvalue _gamecoordinate) (Default|GetHoverSpace (.Game%20State (CallFunction|GetFlipTacToeGameState)) self))
    (if _returnvalue
      (Class|FTTMultiplayerController|HandleSpaceSelect _gamecoordinate))))

(event Input|AxisEvents|InputAxisRotateClockwise
  (params (AxisValue :type Float%20%28single-precision%29))
  (Utilities|MovingCamera
    (:true
      (bind _asbp_default_pawn (Utilities|Casting|CastToBP_DefaultPawn (Game|Player|GetPlayerPawn 0)))
      (Default|RotateClockwise _asbp_default_pawn AxisValue))))

(event Input|AxisEvents|InputAxisPitchUp
  (params (AxisValue :type Float%20%28single-precision%29))
  (Utilities|MovingCamera
    (:true
      (bind _asbp_default_pawn (Utilities|Casting|CastToBP_DefaultPawn (Game|Player|GetPlayerPawn 0)))
      (Default|PitchUp _asbp_default_pawn AxisValue))))

(event Input|AxisEvents|InputAxisZoomIn
  (params (AxisValue :type Float%20%28single-precision%29))
  (bind _asbp_default_pawn (Utilities|Casting|CastToBP_DefaultPawn (Game|Player|GetPlayerPawn 0)))
  (Default|Zoomin _asbp_default_pawn AxisValue))

(fn ConstructionScript)

(fn TickHoverSpace
  (bind (_game_state _bsuccess) (CallFunction|GetFlipTacToeGameState))
  (switch Utilities|FlowControl|Switch|SwitchonPlayerPhase (Variables|Default|GetCurrentPlayerPhase)
    (:Winner
      (Default|SetHoverSpace (.Game%20State (CallFunction|GetFlipTacToeGameState)) false :!label _label))
    (:Loser
      (goto _label))
    (:WaitingForOpponent
      (goto _label))
    (:SelectOpponentPiece
      (Utilities|MovingCamera :!label _label_2
        (:true
          (goto _label))
        (:false
          (if _bsuccess
            (bind (_returnvalue _gamecoordinate) (Default|GetHoverSpace _game_state self))
            (if _returnvalue
              (bind _output_get (LocalVariables|SetHoveredSpace _gamecoordinate))
              (bind _output_get_2 (LocalVariables|SetGameBoard (CallFunction|GetFlipTacToeGameBoard)))
              (if (.IsValid (Class|GameBoard|GetPieceInfoatSpace _output_get_2 _output_get))
                (Utilities|SwitchGamePhase
                  (:Select%20opponent%20piece
                    (Default|SetHoverSpace (.Game%20State (CallFunction|GetFlipTacToeGameState)) (not (Utilities|Array|ContainsItem (Class|GameBoard|GetEmptySpaces (LocalVariables|GetGameBoard)) (LocalVariables|GetHoveredSpace))) (LocalVariables|GetHoveredSpace)))
                  (:Flip%20opponent%20piece
                    (Default|SetHoverSpace (.Game%20State (CallFunction|GetFlipTacToeGameState)) (Utilities|Array|ContainsItem (Class|GameBoard|GetAvailableFlipSpaces (LocalVariables|GetGameBoard) (Variables|Default|GetOpponentSpace)) (LocalVariables|GetHoveredSpace)) (LocalVariables|GetHoveredSpace)))
                  (:Place%20own%20piece
                    (Default|SetHoverSpace (.Game%20State (CallFunction|GetFlipTacToeGameState)) (Utilities|Array|ContainsItem (Class|GameBoard|GetEmptySpaces (LocalVariables|GetGameBoard)) (LocalVariables|GetHoveredSpace)) (LocalVariables|GetHoveredSpace))))
                (else
                  (Utilities|SwitchGamePhase
                    (:Select%20opponent%20piece
                      (Default|SetHoverSpace (.Game%20State (CallFunction|GetFlipTacToeGameState)) false (LocalVariables|GetHoveredSpace)))
                    (:Flip%20opponent%20piece
                      (Default|SetHoverSpace (.Game%20State (CallFunction|GetFlipTacToeGameState)) false (LocalVariables|GetHoveredSpace)))
                    (:Place%20own%20piece
                      (Default|SetHoverSpace (.Game%20State (CallFunction|GetFlipTacToeGameState)) false (LocalVariables|GetHoveredSpace))))))
              (else
                (goto _label)))
            (else
              (goto _label))))))
    (:FlipOpponentPiece
      (goto _label_2))
    (:PlaceOwnPiece
      (goto _label_2))))