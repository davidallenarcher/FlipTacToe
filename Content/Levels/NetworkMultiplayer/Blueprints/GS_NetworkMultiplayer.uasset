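; Game State Blueprint for the network multiplayer level that shows the hovered space on the game board.
; SetHoverSpace relays to a multi event that sets or clears the hover on a cached BP_GameBoard, and a RepNotify coordinate also sets it.
; GetHoverSpace line-traces from a player's deprojected mouse position and has the board convert the hit to a coordinate.
; The older hover getter and local coordinate conversion are stubs.
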(event Custom|SetHoverSpace_Multi
  (params (ShouldHover? :type Boolean) (HoverCoordinate :type Game%20Coordinate%20Structure))
  (if ShouldHover?
    (Default|SetHoveredSpace (CallFunction|GetBPGameBoard) HoverCoordinate)
    (else
      (Default|ClearHoverSpace (CallFunction|GetBPGameBoard)))))

(event EventSetHoverSpace
  (params (ShouldHover? :type Boolean) (HoverCoordinate :type Game%20Coordinate%20Structure))
  (CallFunction|SetHoverSpaceMulti ShouldHover? HoverCoordinate))

(fn ConstructionScript)

(fn GetHoverSpaceOLD
  (params (Player%20Controller :type Player%20Controller%20Object%20Reference)))

(fn OnRepHighlightedCoordinateSpace
  (Default|SetHoveredSpace (CallFunction|GetBPGameBoard) (Variables|Default|GetHighlightedCoordinateSpace)))

(fn WorldCoordinatetoBoardCoordinate
  (params (WorldCoordinate :type Vector))
  (return false ""))

(fn GetBPGameBoard
  (Variables|Default|GetBP_GameBoard
    (:then
      _)
    (:else
      (bind _returnvalue (Class|FTTNetworkGameState|GetGameBoard))
      (bind _asbp_game_board (Utilities|Casting|CastToBP_GameBoard _returnvalue))
      (bind _output_get (Variables|Default|SetBP_GameBoard _asbp_game_board))))
  (return _output_get))

(fn GetHoverSpace
  (params (PlayerController :type Player%20Controller%20Object%20Reference))
  (bind (_worldlocation _worlddirection) (Game|Player|ConvertMouseLocationToWorldSpace PlayerController))
  (bind (_outhit _returnvalue) (Collision|LineTraceByChannel _worldlocation (|(WorldLocation+(WorldDirection*100)) _worldlocation _worlddirection) "TraceTypeQuery1" false 0 "ForOneFrame"))
  (if _returnvalue
    (return (.IsValid? (Default|WorldCoordinatetoBoardCoordinate (CallFunction|GetBPGameBoard) (.Location (Collision|BreakHitResult _outhit)))) (.Board%20Coordinate (Default|WorldCoordinatetoBoardCoordinate (CallFunction|GetBPGameBoard) (.Location (Collision|BreakHitResult _outhit)))))
    (else
      (return false ""))))